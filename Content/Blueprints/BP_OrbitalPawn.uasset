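; BP_OrbitalPawn is an orbital camera pawn that transitions between points of view on a spring arm.
; On BeginPlay it sets the camera manager's maximum view pitch to zero, so the view cannot tilt above horizontal.
; ChangeOrbitalPov plays a timeline that lerps control rotation along the shortest path to the Pov actor's rotation and blends arm length toward that Pov's SpringArmLength.
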(event `self.ReceiveBeginPlay`
  (set `PlayerCameraManager.ViewPitchMax` 0.0 (`GameplayStatics.GetPlayerCameraManager` 0)))

(event `ChangeOrbitalPov`
  (params (Pov :type "/Game/Blueprints/BP_POV Object Reference"))
  ;[0.7154 0.2391 0.849] Change Pov
  (bind (_direction _alpha) (`Timeline|ChangePovTimeline` :!via `PlayFromStart`)
    (:`Update`
      (`Controller.SetControlRotation` (`GameplayStatics.GetPlayerController` 0) (`KismetMathLibrary.RLerp` (`self.GetControlRotation`) (`self.K2_GetActorRotation` Pov) _alpha true))
      (set `SpringArmComponent.TargetArmLength` (`KismetMathLibrary.Lerp` (`SpringArmComponent.TargetArmLength` (`self.SpringArm`)) (`/Game/Blueprints/BP_POV.SpringArmLength` Pov) _alpha) (`self.SpringArm`)))))

(fn `UserConstructionScript`)